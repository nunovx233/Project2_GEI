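; BP_GameHub is a Blueprint that manages the pause menu and the matching input mode for the first player.
; BeginPlay sets game-only input and hides the mouse cursor.
; TogglePause uses a FlipFlop: one call creates WBP_PauseMenu, pauses the game and enables the cursor with game-and-UI input, and the next removes the menu and restores play.
; The FlipFlop alone tracks pause state, so unpausing by other means leaves it out of step.
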(event Custom|TogglePause
  (bind _returnvalue (Game|GetPlayerController 0))
  (bind _returnvalue_2 (Game|GetPlayerController 0))
  (Utilities|FlowControl|FlipFlop
    (:A
      (bind _returnvalue_3 (UserInterface|CreateWidget "/Game/UI/WBP_PauseMenu.WBP_PauseMenu_C"))
      (Variables|Default|SetPauseMenuRef _returnvalue_3)
      (UserInterface|Viewport|AddtoViewport _returnvalue_3 0)
      (Game|SetGamePaused true)
      (Input|SetInputModeGameandUI _returnvalue _returnvalue_3 "DoNotLock" true false)
      (Variables|/Script/Engine.PlayerController|SetbShowMouseCursor _returnvalue true))
    (:B
      (Widget|RemovefromParent (Variables|Default|GetPauseMenuRef))
      (Game|SetGamePaused false)
      (Input|SetInputModeGameOnly _returnvalue_2 false)
      (Variables|/Script/Engine.PlayerController|SetbShowMouseCursor _returnvalue_2 false))))

(event EventBeginPlay
  (bind _returnvalue (Game|GetPlayerController 0))
  (Input|SetInputModeGameOnly _returnvalue false)
  (Variables|/Script/Engine.PlayerController|SetbShowMouseCursor _returnvalue false))

(fn ConstructionScript)