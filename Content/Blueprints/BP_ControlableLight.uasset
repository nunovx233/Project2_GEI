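; BP_ControlableLight is a light Blueprint whose point light is switched on and off through a TogglePowerState event.
; It starts dark by zeroing the PointLight intensity on BeginPlay.
; TogglePowerState takes a State flag and sets both intensity and color, giving bright white when on and zero-intensity black when off.
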(event EventTogglePowerState
  (params (bState :type Boolean))
  (if bState
    (Rendering|Components|Light|SetIntensity (Variables|Default|GetPointLight) 5e+03)
    (Rendering|Components|Light|SetLightColor (Variables|Default|GetPointLight) "(R=1.000000,G=1.000000,B=1.000000,A=1.000000)" true)
    (else
      (Rendering|Components|Light|SetIntensity (Variables|Default|GetPointLight) 0.0)
      (Rendering|Components|Light|SetLightColor :self (Variables|Default|GetPointLight)))))

(event EventBeginPlay
  (Rendering|Components|Light|SetIntensity (Variables|Default|GetPointLight) 0.0))

(fn ConstructionScript)