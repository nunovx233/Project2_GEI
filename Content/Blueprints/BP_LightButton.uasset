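; BP_LightButton is an interactable puzzle button that cycles the color of its puzzle light.
; Overlapping the box with the player pawn shows a text prompt and enables input on the actor; leaving reverses both.
; Pressing E advances a wrapping index through the available colors, updates the light, and asks the PuzzleController to check the sequence.
; GetCurrentColor exposes the selected color.
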(event OnComponentBeginOverlap(Box)
  (params (OverlappedComponent :type Primitive%20Component%20Object%20Reference) (OtherActor :type Actor%20Object%20Reference) (OtherComp :type Primitive%20Component%20Object%20Reference) (OtherBodyIndex :type Integer) (bFromSweep :type Boolean) (SweepResult :type Hit%20Result%20Structure%20%28by%20ref%29))
  (if (== OtherActor (Game|Player|GetPlayerPawn 0))
    (Input|EnableInput (Game|GetPlayerController 0))
    (Rendering|SetVisibility (Variables|Default|GetTextRender) true false)))

(event OnComponentEndOverlap(Box)
  (params (OverlappedComponent :type Primitive%20Component%20Object%20Reference) (OtherActor :type Actor%20Object%20Reference) (OtherComp :type Primitive%20Component%20Object%20Reference) (OtherBodyIndex :type Integer))
  (if (== OtherActor (Game|Player|GetPlayerPawn 0))
    (Input|DisableInput (Game|GetPlayerController 0))
    (Rendering|SetVisibility (Variables|Default|GetTextRender) false false)))

(event Input|KeyboardEvents|E
  (params (Key :type Key%20Structure))
  (:Pressed
    (Variables|Default|SetCurrentColorIndex (Math|Integer|%(Integer) (+ (Variables|Default|GetCurrentColorIndex) 1) (Utilities|Array|Length (Variables|Default|GetAvailableColors))))
    (CallFunction|UpdateLightColor)
    (Default|CheckSequence (Variables|Default|GetPuzzleController))))

(fn ConstructionScript)

(fn UpdateLightColor
  (Rendering|Components|Light|SetLightColor (Variables|Default|GetPuzzleLight) (Utilities|Array|Get(acopy) (Variables|Default|GetAvailableColors) (Variables|Default|GetCurrentColorIndex)) true)
  (return))

(fn GetCurrentColor
  (return (Utilities|Array|Get(acopy) (Variables|Default|GetAvailableColors) (Variables|Default|GetCurrentColorIndex))))