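; Oxygen pickup actor that adds OxygenGained to the main character's CurrentOxygen when BP_MainCharacter overlaps its Box.
; On overlap it prints the amount gained and destroys itself.
; Tick bobs the OxygenGainPickup component on a sine of game time around the Z height cached at BeginPlay, and spins it in yaw scaled by delta time.
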(event OnComponentBeginOverlap(Box)
  (params (OverlappedComponent :type Primitive%20Component%20Object%20Reference) (OtherActor :type Actor%20Object%20Reference) (OtherComp :type Primitive%20Component%20Object%20Reference) (OtherBodyIndex :type Integer) (bFromSweep :type Boolean) (SweepResult :type Hit%20Result%20Structure%20%28by%20ref%29))
  (bind _oxygengained (Variables|Default|GetOxygenGained))
  (bind _asbp_main_character (Utilities|Casting|CastToBP_MainCharacter OtherActor))
  (Variables|/Game/Blueprints/BP_MainCharacter.BP_MainCharacter_C|SetCurrentOxygen _asbp_main_character (+ (Variables|/Game/Blueprints/BP_MainCharacter.BP_MainCharacter_C|GetCurrentOxygen _asbp_main_character) _oxygengained))
  (Development|PrintString (Utilities|String|Append "Oxygen Gained:" (Utilities|String|ToString(Float) _oxygengained)))
  (Actor|DestroyActor))

(event EventBeginPlay
  (Variables|Default|SetInitialZLocation (.Z (Math|Vector|BreakVector (Variables|/Script/Engine.SceneComponent|GetRelativeLocation (Variables|Default|GetOxygenGainPickup))))))

(event EventTick
  (params (DeltaSeconds :type Float%20%28single-precision%29))
  (Transformation|SetRelativeLocation (Variables|Default|GetOxygenGainPickup) (Math|Vector|MakeVector 0.0 0.0 (+ (* (Math|Trig|Sin(Degrees) (* (Utilities|Time|GetGameTimeinSeconds) (Variables|Default|GetFloatSpeed))) (Variables|Default|GetFloatAmplitude)) (Variables|Default|GetInitialZLocation))) false false)
  (Utilities|FlowControl|Sequence
    (:then_1
      (Transformation|AddLocalRotation (Variables|Default|GetOxygenGainPickup) (Math|Rotator|MakeRotator 0.0 0.0 (* (Utilities|Time|GetWorldDeltaSeconds) (Variables|Default|GetRotationSpeed))) false false))))

(fn ConstructionScript)