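; Puzzle controller that opens a door when the colors of its LightButtons match CorrectSequence.
; CheckSequence compares each button in order and exits at the first mismatch.
; A full match plays the Door timeline, which sets Door2 to a fixed rotation, and sends a power-state interface message to EnvironmentalLight.
; It then calls helpers that switch the view to DoorCamera and back to the player pawn.
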(event Custom|OpenDoor
  (Timeline|Door Play
    (:Update
      (Transformation|SetRelativeRotation (Variables|Default|GetDoor2) (Math|Rotator|MakeRotator 0.0 0.0 9e+01) false false))))

(fn ConstructionScript)

(fn CheckSequence
  (for (_array_element _array_index) (Variables|Default|GetLightButtons)
    (bind _colorout (Default|GetCurrentColor _array_element))
    (if (!= _colorout (Utilities|Array|Get(acopy) (Variables|Default|GetCorrectSequence) _array_index))
      (return)))
  (CallFunction|OpenDoor)
  (Class|BPIPowerControl|TogglePowerState(Message) (Variables|Default|GetEnvironmentalLight) true)
  (Utilities|ChangeView
    (:Out
      (Utilities|ChangeViewtoCharacter))))