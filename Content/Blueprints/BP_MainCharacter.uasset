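; BP_MainCharacter is the player character, handling Enhanced Input look, movement, sprint, punch montage with audio, and pause toggling through BP_GameHub.
; A looping timer from BeginPlay depletes oxygen and broadcasts the normalized level.
; Each tick of that timer also overwrites a level PostProcessVolume's settings, ramping vignette and intensity as oxygen runs low.
; At zero oxygen, it pauses the game and prints a death message.
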(event Custom|OxygenDepletion
  ;[0.15 0.15 0.15 0.5] Oxygen Depletion
  (bind _output_get (Variables|Default|SetCurrentOxygen (- (Variables|Default|GetCurrentOxygen) (Variables|Default|GetOxygenDepletionRate))))
  (Default|CallOnOxygenChanged (/ _output_get (Variables|Default|GetMaxOxygen)))
  (CallFunction|UpdateOxygenEffects)
  (bind _output_get_2 (Variables|Default|SetisDead (<= _output_get 0.0)))
  (if _output_get_2
    (Game|SetGamePaused true)
    (Development|PrintString "You died")))

(event Custom|OxygenTimeOut
  ;[0.15 0.15 0.15 0.5] Oxygen Depletion
  (Utilities|Time|SetTimerbyEvent (delegate Custom|OxygenDepletion) 6.0 true))

(event Input|EnhancedActionEvents|EnhancedInputActionIA_Move
  (params (ActionValue :type Vector%202D%20Structure) (ElapsedSeconds :type Float%20%28double-precision%29) (TriggeredSeconds :type Float%20%28double-precision%29) (InputAction :type Input%20Action%20Object%20Reference :default "/Game/Characters/Inputs/IA_Move.IA_Move"))
  (bind _returnvalue (Pawn|GetControlRotation :!class /Script/Engine.Pawn))
  ;[0.15 0.15 0.15 0.5] Movement
  (Pawn|Input|AddMovementInput (Math|Vector|GetForwardVector (Math|Rotator|MakeRotator 0.0 0.0 (.yaw _returnvalue))) (.y ActionValue) false)
  (Pawn|Input|AddMovementInput (Math|Vector|GetRightVector (Math|Rotator|MakeRotator 0.0 0.0 (.yaw _returnvalue))) (.x ActionValue) false))

(event Input|EnhancedActionEvents|EnhancedInputActionIA_Look
  (params (ActionValue :type Vector%202D%20Structure) (ElapsedSeconds :type Float%20%28double-precision%29) (TriggeredSeconds :type Float%20%28double-precision%29) (InputAction :type Input%20Action%20Object%20Reference :default "/Game/Characters/Inputs/IA_Look.IA_Look"))
  ;[0.15 0.15 0.15 0.5] Camera Movement
  (Pawn|Input|AddControllerYawInput (* (.x ActionValue) (Utilities|Time|GetWorldDeltaSeconds) (Variables|Default|GetBase%20Look%20Rate)))
  (Pawn|Input|AddControllerPitchInput (* (.y ActionValue) (Utilities|Time|GetWorldDeltaSeconds) (Variables|Default|GetBase%20Look%20Rate))))

(event Input|EnhancedActionEvents|EnhancedInputActionIA_Sprint
  (params (ActionValue :type Boolean) (ElapsedSeconds :type Float%20%28double-precision%29) (TriggeredSeconds :type Float%20%28double-precision%29) (InputAction :type Input%20Action%20Object%20Reference :default "/Game/Characters/Inputs/IA_Sprint.IA_Sprint"))
  (bind _charactermovement (Variables|Character|GetCharacterMovement))
  ;[0.15 0.15 0.15 0.5] Runnig
  (:Started
    (Variables|/Script/Engine.CharacterMovementComponent|SetMaxWalkSpeed _charactermovement 6e+02))
  (:Completed
    (Variables|/Script/Engine.CharacterMovementComponent|SetMaxWalkSpeed _charactermovement 3e+02)))

(event Input|EnhancedActionEvents|EnhancedInputActionIA_PauseMenu
  (params (ActionValue :type Boolean) (ElapsedSeconds :type Float%20%28double-precision%29) (TriggeredSeconds :type Float%20%28double-precision%29) (InputAction :type Input%20Action%20Object%20Reference :default "/Game/Characters/Inputs/IA_PauseMenu.IA_PauseMenu"))
  ;[0.15 0.15 0.15 0.5] TogglePause
  (:Triggered
    (bind _asbp_game_hub (Utilities|Casting|CastToBP_GameHub (HUD|GetHUD (Game|GetPlayerController 0)) :!label _label))
    (Default|TogglePause _asbp_game_hub))
  (:Started
    (goto _label)))

(event Input|EnhancedActionEvents|EnhancedInputActionIA_Attack
  (params (ActionValue :type Boolean) (ElapsedSeconds :type Float%20%28double-precision%29) (TriggeredSeconds :type Float%20%28double-precision%29) (InputAction :type Input%20Action%20Object%20Reference :default "/Game/Characters/Inputs/IA_Attack.IA_Attack"))
  ;[0.15 0.15 0.15 0.5] Attack
  (:Started
    (Animation|PlayAnimMontage "/Game/Characters/Animations/AM_Punch1.AM_Punch1" 1.0 "None")
    (Audio|Components|Audio|Play (Variables|Default|GetAudio) 0.0)))

(event EventBeginPlay
  (CallFunction|OxygenTimeOut)
  (Input|AddMappingContext (PlayerController|LocalPlayerSubsystems|GetEnhancedInputLocalPlayerSubsystem (Game|GetPlayerController 0)) (Variables|Default|GetMapping%20Context) 0 "(bIgnoreAllPressedKeysUntilRelease=True,bForceImmediately=False,bNotifyUserSettings=False)"))

(fn ConstructionScript)

(fn UpdateOxygenEffects
  (bind _currentoxygen (Variables|Default|GetCurrentOxygen))
  (bind _returnvalue (Math|Float|MapRangeClamped _currentoxygen 4e+01 1e+01 0.0 2.0))
  (bind _returnvalue_2 (Actor|GetActorOfClass "/Script/Engine.PostProcessVolume"))
  (Utilities|IsValid _returnvalue_2
    (:Is%20Valid
      (Variables|/Script/Engine.PostProcessVolume|SetSettings _returnvalue_2 (Utilities|Struct|MakePostProcessSettings "(R=0.991566,G=1.000000,B=0.991054,A=1.000000)" _returnvalue _returnvalue))
      (return))))